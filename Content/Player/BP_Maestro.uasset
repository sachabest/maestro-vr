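; BP_Maestro is a motion-controller player Blueprint that tracks a conducting state and can launch cubes.
; The left trigger sets Conducting while held, but the Tick branch on it is still empty.
; Emit spawns a BasicCube at the held cube's location, starts its motion and applies an impulse from GetControllerDelta.
; Emit is not called here, and GetControllerDelta's controller-minus-actor offset is left unconnected.
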(event EventBeginPlay
  (|CallParentFunction))

(event Collision|EventActorBeginOverlap
  (params (OtherActor :type Actor%20Object%20Reference)))

(event EventTick
  (params (DeltaSeconds :type Float%20%28single-precision%29))
  (|CallParentFunction DeltaSeconds)
  (if (Variables|Default|GetbConducting)
    _))

(event Input|KeyboardEvents|MotionControllerLeftTrigger
  (params (Key :type Key%20Structure :default "AnyKey"))
  (:Pressed
    (Variables|Default|SetbConducting true))
  (:Released
    (Variables|Default|SetbConducting false)))

(fn ConstructionScript
  (|CallParentFunction))

(fn Emit
  (bind _returnvalue (Game|SpawnActorfromClass "/Game/Throwables/BasicCube.BasicCube_C" (Math|Conversions|ToTransform(Vector) (Transformation|GetWorldLocation (Variables|/Game/Throwables/BasicCube.BasicCube_C|GetCube (Variables|Default|GetaHeldCube)))) "AlwaysSpawn" 0 0))
  (Default|OnMotionStart _returnvalue)
  (Physics|AddImpulse (Variables|/Game/Throwables/BasicCube.BasicCube_C|GetCube _returnvalue) (Utilities|GetControllerDelta) "None" false))